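; Pooled primary-attack projectile for the Zinx character that deals damage through the Gameplay Ability System.
; A hit plays the impact effect pack, while an overlap with any actor but its owner also applies the primary attack damage effect to that actor.
; Lifespan expiry plays a separate effect, and all three outcomes return it to the actor pool.
; Leaving the pool caches the ability system component passed in the pop data.
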(event OnComponentHit(CollisionComponent)
  (params (HitComponent :type Primitive%20Component%20Object%20Reference) (OtherActor :type Actor%20Object%20Reference) (OtherComp :type Primitive%20Component%20Object%20Reference) (NormalImpulse :type Vector :default "0, 0, 0") (Hit :type Hit%20Result%20Structure%20%28by%20ref%29))
  (Class|RPGBFLMainFunctions|PlayEffectPackatLocation (Variables|Default|GetImpact) self 0 "Instant" (Math|Transform|MakeTransform (.ImpactPoint (Collision|BreakHitResult Hit)) (Transformation|GetActorRotation) "1.000000,1.000000,1.000000"))
  (Class|ActorPoolWorldSubsystem|AddActortoPool (Subsystems|GetActorPoolWorldSubsystem) self))

(event OnComponentBeginOverlap(CollisionComponent)
  (params (OverlappedComponent :type Primitive%20Component%20Object%20Reference) (OtherActor :type Actor%20Object%20Reference) (OtherComp :type Primitive%20Component%20Object%20Reference) (OtherBodyIndex :type Integer) (bFromSweep :type Boolean) (SweepResult :type Hit%20Result%20Structure%20%28by%20ref%29))
  (if (!= OtherActor (Components|GetOwner))
    (Class|RPGBFLMainFunctions|PlayEffectPackatLocation (Variables|Default|GetImpact) self 0 "Instant" (Math|Transform|MakeTransform (.ImpactPoint (Collision|BreakHitResult SweepResult)) (Transformation|GetActorRotation) "1.000000,1.000000,1.000000"))
    (GameplayEffects|ApplyGameplayEffectToTarget :self (Variables|Default|GetASC) :GameplayEffectClass "/Game/Characters/Global/GE/GE_PrimaryAttackDamage.GE_PrimaryAttackDamage_C" :Target (Ability|GetAbilitySystemComponent OtherActor))
    (Class|ActorPoolWorldSubsystem|AddActortoPool (Subsystems|GetActorPoolWorldSubsystem) self)))

(event EventBeginPlay)

(event Collision|EventActorBeginOverlap
  (params (OtherActor :type Actor%20Object%20Reference)))

(event EventTick
  (params (DeltaSeconds :type Float%20%28single-precision%29)))

(event EventOnPoolLeft
  (params (PopData :type Actor%20Pop%20Data%20Structure%20%28by%20ref%29))
  (|CallParentFunction PopData)
  (bind _asability_system_component (Utilities|Casting|CastToAbilitySystemComponent (Utilities|Struct|BreakActorPopData PopData)))
  (Variables|Default|SetASC _asability_system_component))

(event EventOnPoolEntered
  (|CallParentFunction))

(event EventLifeSpanExpired
  (Class|RPGBFLMainFunctions|PlayEffectPackatLocation (Variables|Default|GetLifetimeExceededEffect) self 0 "Instant" (Math|Transform|MakeTransform (Transformation|GetActorLocation) (Transformation|GetActorRotation) "1.000000,1.000000,1.000000"))
  (Class|ActorPoolWorldSubsystem|AddActortoPool (Subsystems|GetActorPoolWorldSubsystem) self))

(fn ConstructionScript
  (|CallParentFunction))