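; Pooled ricochet projectile for Zinx that applies primary attack damage and bounces between nearby actors.
; Each overlap with an ability-system actor applies the damage effect, then sphere-traces for another target, excluding the owner and prior hits.
; It homes onto that target and restarts its lifetime.
; Blocking hits, lifetime expiry, no target or reaching max bounces play destroyed FX and return it to the pool, where bounce state resets.
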(event OnComponentHit(CollisionComponent)
  (params (HitComponent :type Primitive%20Component%20Object%20Reference) (OtherActor :type Actor%20Object%20Reference) (OtherComp :type Primitive%20Component%20Object%20Reference) (NormalImpulse :type Vector :default "0, 0, 0") (Hit :type Hit%20Result%20Structure%20%28by%20ref%29))
  (CallFunction|DoneBouncing))

(event OnComponentBeginOverlap(CollisionComponent)
  (params (OverlappedComponent :type Primitive%20Component%20Object%20Reference) (OtherActor :type Actor%20Object%20Reference) (OtherComp :type Primitive%20Component%20Object%20Reference) (OtherBodyIndex :type Integer) (bFromSweep :type Boolean) (SweepResult :type Hit%20Result%20Structure%20%28by%20ref%29))
  (if (!= OtherActor (Components|GetOwner))
    (CallFunction|OnOverlap OtherActor)))

(event Custom|DoneBouncing
  (Class|RPGBFLMainFunctions|PlayEffectPackatLocation (Variables|Default|GetDestroyedFX) (Components|GetOwner) 0 "Instant" (Math|Transform|MakeTransform (Transformation|GetActorLocation) (Transformation|GetActorRotation) "1.000000,1.000000,1.000000"))
  (Class|RPGProjectile|ReturnProjectiletoPool))

(event EventBeginPlay)

(event Collision|EventActorBeginOverlap
  (params (OtherActor :type Actor%20Object%20Reference)))

(event EventTick
  (params (DeltaSeconds :type Float%20%28single-precision%29)))

(event EventLifeSpanExpired
  (CallFunction|DoneBouncing))

(event EventOnPoolEntered
  (|CallParentFunction)
  (Variables|/Script/Engine.ProjectileMovementComponent|SetHomingTargetComponent (Variables|Default|GetProjectileMovementComponent) 0)
  (Variables|Default|SetCurrentBounces 0)
  (Utilities|Array|Clear (Variables|Default|GetHitActors)))

(fn ConstructionScript)

(fn SetNewHomingTarget
  (params (NewTarget :type Actor%20Object%20Reference))
  (bind _lifetimehandler (Variables|Default|GetLifetimeHandler))
  (bind _projectilemovementcomponent (Variables|Default|GetProjectileMovementComponent))
  (Variables|/Script/Engine.MovementComponent|SetVelocity _projectilemovementcomponent (* (Math|Vector|Normalize (- (Transformation|GetActorLocation NewTarget) (Transformation|GetActorLocation))) 1e+03))
  (Variables|/Script/Engine.ProjectileMovementComponent|SetHomingTargetComponent _projectilemovementcomponent (Actor|GetComponentbyClass NewTarget "/Script/Engine.SceneComponent"))
  (Class|LifetimeHandlerComponent|StopLifetime _lifetimehandler)
  (Class|LifetimeHandlerComponent|StartLifetime _lifetimehandler))

(fn TryGetValidNewTarget
  (params (LastTarget :type Actor%20Object%20Reference))
  (bind _returnvalue (Transformation|GetActorLocation))
  (bind _output_get (LocalVariables|SetTempArray (Utilities|Array|MakeArray (Components|GetOwner))))
  (Utilities|Array|AppendArray _output_get (Variables|Default|GetHitActors))
  (bind (_outhit _returnvalue_2) (Collision|SphereTraceForObjects _returnvalue _returnvalue 8e+02 (Utilities|Array|MakeArray "ObjectTypeQuery3" "ObjectTypeQuery7") false (LocalVariables|GetTempArray) "None"))
  (return _outhit _returnvalue_2))

(fn OnOverlap
  (params (OtherActor :type Actor%20Object%20Reference))
  (bind _returnvalue (Ability|GetAbilitySystemComponent OtherActor))
  (Utilities|IsValid _returnvalue
    (:Is%20Valid
      (Utilities|Array|Add (Variables|Default|GetHitActors) OtherActor)
      (GameplayEffects|ApplyGameplayEffectToTarget :self (Ability|GetAbilitySystemComponent (Components|GetOwner)) :GameplayEffectClass "/Game/Characters/Global/GE/GE_PrimaryAttackDamage.GE_PrimaryAttackDamage_C" :Target _returnvalue)
      (bind (_hitresult _bfoundnewtarget) (CallFunction|TryGetValidNewTarget OtherActor))
      (if _bfoundnewtarget
        (if (< (Variables|Default|GetCurrentBounces) (Variables|Default|GetMaxBounces))
          (Math|Integer|IncrementInt (Variables|Default|GetCurrentBounces)
            (:%20%20
              (CallFunction|SetNewHomingTarget (.HitActor (Collision|BreakHitResult _hitresult)))))
          (else
            (CallFunction|DoneBouncing)))
        (else
          (CallFunction|DoneBouncing))))))