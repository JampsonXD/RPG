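; BP_VFX_Lightning is a self-running lightning effect actor that plays a timed launch and hit sequence with visuals and sound.
; On BeginPlay it waits briefly, then plays the launch sound and activates the muzzle effect component.
; A moment later it activates the hit effect component with its impact sound, each sound spawned at its component's location.
; The actor destroys itself after a final delay.
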(event EventBeginPlay
  (bind _ns_lightning_hit (Variables|Default|GetNS_Lightning_Hit))
  (Utilities|FlowControl|Delay 1.0)
  (Audio|SpawnSoundatLocation "/Game/Vefects/Anime_VFX/Shared/Audio/SFX_Lightning_Launch_Cue.SFX_Lightning_Launch_Cue" (Transformation|GetWorldLocation (Variables|Default|GetNS_Lightning_Muzzle)) "0, 0, 0" 1.0 1.0 0.0 0 0)
  (Components|Activation|Activate (Variables|Default|GetNS_Lightning_Muzzle) false)
  (Utilities|FlowControl|Delay 0.1)
  (Components|Activation|Activate _ns_lightning_hit false)
  (Audio|SpawnSoundatLocation "/Game/Vefects/Anime_VFX/Shared/Audio/SFX_Lightning_Hit_Cue.SFX_Lightning_Hit_Cue" (Transformation|GetWorldLocation _ns_lightning_hit) "0, 0, 0" 1.0 1.0 0.0 0 0)
  (Utilities|FlowControl|Delay 2.0)
  (Actor|DestroyActor))

(fn ConstructionScript)