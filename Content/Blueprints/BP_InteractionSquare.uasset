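; Test-style interactable, poolable square that grants a stack of its item to the interacting actor's inventory.
; PreInteract rejects interaction system components already in progress; Interact registers the component, starts a duration timer, randomizes the cube's emissive color and plays a pickup effect if an inventory exists.
; PostInteract prints the end state, releases the component and plays a respawn effect.
; Pool callbacks enable box physics on leaving and disable it on entering.
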(event Custom|CleanupInteraction
  (Class|InteractableInterface|PostInteract (stale EventInteract InteractInfo) "EndSuccessful"))

(event EventOnPoolLeft
  (params (PopData :type Actor%20Pop%20Data%20Structure%20%28by%20ref%29))
  (Physics|SetSimulatePhysics (Variables|Default|GetBox) true))

(event EventInteract
  (params (InteractInfo :type Interact%20Info%20Structure))
  (bind (_interactingactor _interactinginteractionsystemcomponent) (Utilities|Struct|BreakInteractInfo InteractInfo))
  (bind _returnvalue (Class|BFLInventory|GetInventorySystemComponent _interactingactor))
  (Utilities|Array|Add (Variables|Default|GetInteractingISCs) _interactinginteractionsystemcomponent)
  (bind _returnvalue_2 (Utilities|Time|SetTimerbyEvent (EventDispatchers|CreateEvent :!event Custom|CleanupInteraction) (Variables|Default|GetInteractionDuration)))
  (Variables|Default|SetTimerHandle _returnvalue_2)
  (bind _returnvalue_3 (Rendering|Material|CreateDynamicMaterialInstance (Variables|Default|GetCube) 0 0 "None" :!class /Script/Engine.PrimitiveComponent))
  (Rendering|Material|SetVectorParameterValue _returnvalue_3 "Emissive_Color" (Utilities|Struct|MakeLinearColor (Math|Random|RandomFloat) (Math|Random|RandomFloat) (Math|Random|RandomFloat) 1.0) :!class /Script/Engine.MaterialInstanceDynamic)
  (Utilities|IsValid _returnvalue
    (:Is%20Valid
      (Class|InventorySystemComponent|AddItem _returnvalue (Variables|Default|GetItem) 30 false)
      (Class|RPGBFLMainFunctions|PlayEffectPackatLocation (Variables|Default|GetPickupEffectPack) self 0 "Instant" (Math|Transform|MakeTransform (Transformation|GetActorLocation) "0, 0, 0" "1.000000,1.000000,1.000000")))))

(event EventOnPoolEntered
  (Physics|SetSimulatePhysics (Variables|Default|GetBox) false))

(event EventPostInteract
  (params (InteractInfo :type Interact%20Info%20Structure) (EndState :type EInteractionEndState%20Enum :default "None"))
  (Development|PrintText (Utilities|Text|FormatText "Interacting Actor {1} : {2}" (Utilities|Struct|BreakInteractInfo InteractInfo) (Utilities|String|EnumtoString EndState)))
  (Utilities|Array|RemoveItem (Variables|Default|GetInteractingISCs) (.InteractingInteractionSystemComponent (Utilities|Struct|BreakInteractInfo InteractInfo)))
  (Class|RPGBFLMainFunctions|PlayEffectPackatLocation (Variables|Default|GetRespawnEffectPack) self 0 "Instant" (Math|Transform|MakeTransform (Transformation|GetActorLocation) "0, 0, 0" "1.000000,1.000000,1.000000")))

(fn ConstructionScript)

(fn PreInteract
  (params (InteractInfo :type Interact%20Info%20Structure))
  (return (not (Utilities|Array|ContainsItem (Variables|Default|GetInteractingISCs) (.InteractingInteractionSystemComponent (Utilities|Struct|BreakInteractInfo InteractInfo))))))