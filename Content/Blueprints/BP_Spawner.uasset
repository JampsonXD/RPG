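; BP_Spawner is a spawner Blueprint that requests pooled actors at its own location and rotation.
; RequestSpawnActors checks for a valid class and positive amount, then rebuilds the pop data with the spawner's transform, keeping the caller's other fields.
; SpawnActor passes the request to ActorPoolWorldSubsystem instead of spawning directly.
; Each request yields one pool call, as Amount is only validated and Delay is unused.
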(event Custom|RequestSpawnActors
  (params (ActorClass :type Actor%20Class%20Reference) (PopData :type Actor%20Pop%20Data%20Structure%20%28by%20ref%29) (Amount :type Integer) (Delay :type Float%20%28double-precision%29))
  (bind (_owner _instigator _location _velocity _rotation _optionalobject _optionalobject2 _optionalgameplaytags _magnitude _optionalmagnitude) (Utilities|Struct|BreakActorPopData PopData))
  (if (CallFunction|IsValidRequest ActorClass Amount)
    (CallFunction|SpawnActor ActorClass (Utilities|Struct|MakeActorPopData _owner _instigator (Transformation|GetActorLocation) _velocity (Transformation|GetActorRotation) _optionalobject _optionalobject2 _optionalgameplaytags _magnitude _optionalmagnitude))))

(fn ConstructionScript)

(fn SpawnActor
  (params (ActorClass :type Actor%20Class%20Reference) (PopData :type Actor%20Pop%20Data%20Structure%20%28by%20ref%29))
  (Class|ActorPoolWorldSubsystem|RequestActorfromPool (Subsystems|GetActorPoolWorldSubsystem) ActorClass PopData))

(fn IsValidRequest
  (params (ActorClass :type Actor%20Class%20Reference) (Amount :type Integer))
  (return (and (Utilities|IsValidClass ActorClass) (> Amount 0))))