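; Player character Blueprint with first-person camera that integrates sensing, interaction, inventory, gameplay ability and quest systems, with extensive debug printing.
; Sprint, jump and death events set gameplay status tags; death also ragdolls the mesh and disables input, and aiming drives an FOV timeline.
; Equipment additions spawn and initialize weapon actors, whose mesh sockets are exposed by lookup.
; Debug helpers print attributes, sensed actors and quest definitions.
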(event CurrentInteractingActorChanged(InteractionSystemComponent)
  (params (NewActor :type Actor%20Object%20Reference) (OldActor :type Actor%20Object%20Reference))
  (Development|PrintString (Utilities|String|ToString(Text) (Utilities|Text|FormatText "New Interacting Actor :  {X} 
Old Interacting Actor :  {Y}" NewActor OldActor))))

(event OnActorSensed(SensingSystemComponent)
  (params (SensedActor :type Actor%20Object%20Reference))
  (Development|PrintText (Utilities|Text|FormatText "{x} Sensed" SensedActor) true true "(R=0.000000,G=0.660000,B=1.000000,A=1.000000)" 5.0))

(event OnActorLost(SensingSystemComponent)
  (params (LostActor :type Actor%20Object%20Reference))
  (Development|PrintText (Utilities|Text|FormatText "{x} Lost Sense" LostActor) true true "(R=0.000000,G=0.660000,B=1.000000,A=1.000000)" 5.0))

(event Custom|OnFOVChange
  (params (bAiming :type Boolean))
  (if bAiming
    (bind _fov (Timeline|FOV Play)
      (:Update
        (Camera|SetFieldOfView (Variables|Default|GetFirstPersonCamera) _fov)))
    (else
      (Timeline|FOV Reverse))))

(event Input|EnhancedActionEvents|EnhancedInputActionIA_Sprint
  (params (ActionValue :type Boolean) (ElapsedSeconds :type Float%20%28double-precision%29) (TriggeredSeconds :type Float%20%28double-precision%29) (InputAction :type Input%20Action%20Object%20Reference :default "/Game/Characters/Global/Inputs/IA_Sprint.IA_Sprint"))
  (bind _self self)
  (:Started
    (Class|RPGBFLMainFunctions|AddLooseGameplayTagstoActor _self "(GameplayTags=((TagName=\"Status.Running\")))")
    (Development|PrintText "Started Sprinting"))
  (:Completed
    (Class|RPGBFLMainFunctions|RemoveLooseGameplayTagstoActor _self "(GameplayTags=((TagName=\"Status.Running\")))")
    (Development|PrintText "Stopped Sprinting")))

(event EventInteract
  (params (InteractInfo :type Interact%20Info%20Structure))
  (Class|InteractableInterface|PostInteract InteractInfo "EndSuccessful"))

(event EventPostInteract
  (params (InteractInfo :type Interact%20Info%20Structure) (EndState :type EInteractionEndState%20Enum :default "None")))

(event EventBeginPlay
  (Class|SensingSystemComponent|InitializeSensingComponent (Variables|Default|GetSensing%20System%20Component) self))

(event EventOnJumped
  (Class|RPGBFLMainFunctions|AddLooseGameplayTagstoActor self "(GameplayTags=((TagName=\"Status.Jumping\")))"))

(event EventOnLanded
  (params (Hit :type Hit%20Result%20Structure%20%28by%20ref%29))
  (Class|RPGBFLMainFunctions|RemoveLooseGameplayTagstoActor self "(GameplayTags=((TagName=\"Status.Jumping\")))"))

(event EventDeathEvent
  (bind _mesh (Variables|Character|GetMesh))
  (Class|RPGBFLMainFunctions|AddLooseGameplayTagstoActor self "(GameplayTags=((TagName=\"Status.Dead\")))")
  (Physics|SetSimulatePhysics _mesh true)
  (Collision|SetCollisionEnabled _mesh "PhysicsOnly")
  (bind _asplayer_controller (Utilities|Casting|CastToPlayerController (Pawn|GetController)))
  (Input|DisableInput _asplayer_controller))

(event Input|KeyboardEvents|NumPadSeven
  (params (Key :type Key%20Structure :default "None"))
  (:Pressed
    (CallFunction|PrintQuestDefInformation)))

(fn ConstructionScript)

(fn PrintAttribute
  (params (Attribute :type Gameplay%20Attribute%20Structure))
  (Development|PrintString (Utilities|String|ToString(Text) (Utilities|Text|FormatText "{Name}: {attribute}" (Utilities|Struct|BreakGameplayAttribute Attribute) (.ReturnValue (Ability|Attribute|GetFloatAttributefromAbilitySystemComponent (Ability|GetAbilitySystemComponent self) Attribute)))) true true "(R=0.000000,G=0.660000,B=1.000000,A=1.000000)" 0.0))

(fn PreInteract
  (params (InteractInfo :type Interact%20Info%20Structure))
  (Development|PrintText (Utilities|Text|FormatText "{RequestActor} is saying hi!" (Utilities|GetDisplayName (.InteractingActor (Utilities|Struct|BreakInteractInfo InteractInfo)))))
  (return false))

(fn PrintSensingActors
  (for (_array_element _array_index) (Class|SensingSystemComponent|GetSensingActors (Variables|Default|GetSensing%20System%20Component))
    (Development|PrintText (Utilities|Text|FormatText "{z} : {x}" _array_index _array_element) true true "(R=0.000000,G=0.660000,B=1.000000,A=1.000000)" 5.0)))

(fn GetMouseX
  (return (Class|Actor|GetInputAxisKeyValue)))

(fn GetMouseY
  (return (Class|Actor|GetInputAxisKeyValue)))

(fn OnEquipmentSlotChanged
  (params (EquippedSlotData :type Equipped%20Slot%20Structure) (Item :type Item%20Object%20Reference) (ChangeType :type EEquipmentSlotChangeType%20Enum :default "None"))
  (switch Utilities|FlowControl|Switch|SwitchonEEquipmentSlotChangeType ChangeType
    (:Added
      (if (== (.SlotType (Utilities|Struct|BreakEquippedSlot EquippedSlotData)) "Weapon")
        (bind _returnvalue (Game|SpawnActorfromClass (Variables|/Script/InventorySystem.Item|GetItemInstanceClass Item) (Math|Transform|MakeTransform "0, 0,-10000.000000" "0, 0, 0" "1.000000,1.000000,1.000000") "Undefined" (Class|InventorySystemComponent|GetOwningActor (Class|RPGCharacter|GetInventorySystemComponent)) 0))
        (Class|EquippableItemInterface|SetupItem(Message) _returnvalue (Utilities|Struct|MakeItemSetupData Item (Class|BFLInventory|GetInventorySystemComponent self) self (Class|InventorySystemComponent|GetItemStateData (Class|RPGCharacter|GetInventorySystemComponent) Item)))
        (Utilities|Array|Add (Variables|Default|GetWeaponActors) _returnvalue)))))

(fn GetWeaponSocketLocation
  (params (InSocketName :type Name))
  (if (Class|RPGPlayerCharacter|IsValidWeaponSlot (Variables|Default|GetCurrentWeaponEquipSlot))
    (return (Transformation|GetSocketTransform (Actor|GetComponentbyClass (Utilities|Array|Get(acopy) (Variables|Default|GetWeaponActors) (Variables|Default|GetCurrentWeaponEquipSlot)) "/Script/Engine.SkeletalMeshComponent") InSocketName "RTS_World"))))

(fn IsDead
  (return (GameplayTags|HasMatchingGameplayTag (Class|RPGCharacter|GetRPGAbilitySystemComponent) "(TagName=\"Status.Dead\")")))

(fn PrintQuestDefInformation
  (for _array_element (Class|QuestSubsystem|GetQuestDefinitions (Subsystems|GetQuestSubsystem))
    (LocalVariables|SetTemp "")
    (for _array_element_2 (.Objectives (Utilities|Struct|BreakQuest _array_element))
      (for _array_element_3 (Utilities|Struct|BreakObjective _array_element_2)
        (LocalVariables|SetTemp (Utilities|String|Append (LocalVariables|GetTemp) (Utilities|String|ToString(Text) (Utilities|Text|FormatText "Task Id: {0} 
Task Title: {1} 
" (.Id (Utilities|Struct|BreakTask _array_element_3)) (.Title (Utilities|Struct|BreakTask _array_element_3))))))))
    (Development|PrintString (Utilities|String|Append (Utilities|String|ToString(Text) (Utilities|Text|FormatText "Quest Id: {0} 
Quest Title: {1} 
Quest Description: {2} 
" (.Id (Utilities|Struct|BreakQuest _array_element)) (.Title (Utilities|Struct|BreakQuest _array_element)) (.Description (Utilities|Struct|BreakQuest _array_element)))) (LocalVariables|GetTemp)))))