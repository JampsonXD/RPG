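; Projectile lifetime rule that ends after the time needed to cover a set Distance at a constant Speed.
; Initialize guards against a zero Speed, then starts a one-shot timer lasting Distance divided by Speed, avoiding per-frame distance tracking.
; TimerElapsed signals LifetimeCompleted, and Deinitialize invalidates the timer handle.
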(event EventInitialize
  (params (Actor :type Actor%20Object%20Reference))
  (CallFunction|DividebyZeroCheck)
  (bind _returnvalue (Utilities|Time|SetTimerbyEvent (EventDispatchers|CreateEvent :!event TimerElapsed) (/ (Variables|Default|GetDistance) (Variables|Default|GetSpeed))))
  (Variables|Default|SetTimerHandle _returnvalue))

(event EventDeinitialize
  (Utilities|Time|InvalidateTimerHandle (Variables|Default|GetTimerHandle)))

(fn TimerElapsed
  (Class|LifetimeChecker|LifetimeCompleted))

(fn DividebyZeroCheck
  (if (== (Variables|Default|GetSpeed) 0.0)
    (Variables|Default|SetSpeed 1.0)))