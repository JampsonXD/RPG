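; Projectile lifetime object that ends once a watched actor has traveled a set distance.
; Initialize records the starting location, then each Tick adds the length moved since the last sample to an accumulated path distance and completes when it reaches the criteria.
; The watched actor is a soft object reference, and if it is invalid on Tick, the object prints a warning and completes the lifetime immediately.
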(event EventInitialize
  (params (Actor :type Actor%20Object%20Reference))
  (Variables|Default|SetDistanceTraveled 0.0)
  (Variables|Default|SetLastLocation (CallFunction|GetLastActorLocation)))

(event EventDeinitialize
  (Variables|Default|SetDistanceTraveled 0.0))

(event EventTick
  (params (DeltaTime :type Float%20%28single-precision%29))
  (Utilities|IfActorIsValid
    (:Valid
      (CallFunction|UpdateDistance)
      (CallFunction|CheckDistanceCriteriaMet))
    (:NotValid
      (Development|PrintString self (Utilities|String|ToString(Text) (Utilities|Text|FormatText "Watching Actor for {This} is invalid! Ending Lifetime..." self)))
      (Class|LifetimeChecker|LifetimeCompleted))))

(fn GetLastActorLocation
  (return (Transformation|GetActorLocation (Utilities|ResolveSoftReference (Variables|Default|GetWatchingActor)))))

(fn UpdateDistance
  (LocalVariables|SetTempLocation (Variables|Default|GetLastLocation))
  (bind _output_get (Variables|Default|SetLastLocation (CallFunction|GetLastActorLocation)))
  (Variables|Default|SetDistanceTraveled (+ (Math|Vector|VectorLength (- (LocalVariables|GetTempLocation) _output_get)) (Variables|Default|GetDistanceTraveled))))

(fn CheckDistanceCriteriaMet
  (if (>= (Variables|Default|GetDistanceTraveled) (Variables|Default|GetDistanceCriteria))
    (Class|LifetimeChecker|LifetimeCompleted)))