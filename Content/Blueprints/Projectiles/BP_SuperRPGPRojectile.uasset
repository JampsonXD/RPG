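; Pooled RPG gun projectile that plays impact effects, pushes physics bodies and damages targets through GAS.
; On leaving the pool it takes the shooter's ability system component and gun data from the pop data.
; Blocking hits and non-owner overlaps play effects, add velocity-times-mass impulse and notify the actor, but only overlaps apply the gameplay effect container.
; Impacts and lifespan expiry return it to the actor pool subsystem.
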(event OnComponentBeginOverlap(CollisionComponent)
  (params (OverlappedComponent :type Primitive%20Component%20Object%20Reference) (OtherActor :type Actor%20Object%20Reference) (OtherComp :type Primitive%20Component%20Object%20Reference) (OtherBodyIndex :type Integer) (bFromSweep :type Boolean) (SweepResult :type Hit%20Result%20Structure%20%28by%20ref%29))
  (Utilities|IsValidOverlap OtherActor
    (:ValidOverlap
      (CallFunction|PlayImpactEffect SweepResult)
      (CallFunction|AddImpulse SweepResult)
      (CallFunction|ApplyImpactDamage OtherActor SweepResult)
      (Class|DamageableInterface|OnPointDamage(Message) OtherActor)
      (Class|ActorPoolWorldSubsystem|AddActortoPool (Subsystems|GetActorPoolWorldSubsystem) self))))

(event OnComponentHit(CollisionComponent)
  (params (HitComponent :type Primitive%20Component%20Object%20Reference) (OtherActor :type Actor%20Object%20Reference) (OtherComp :type Primitive%20Component%20Object%20Reference) (NormalImpulse :type Vector :default "0, 0, 0") (Hit :type Hit%20Result%20Structure%20%28by%20ref%29))
  (CallFunction|PlayImpactEffect Hit)
  (CallFunction|AddImpulse Hit)
  (Class|DamageableInterface|OnPointDamage(Message) OtherActor)
  (Class|ActorPoolWorldSubsystem|AddActortoPool (Subsystems|GetActorPoolWorldSubsystem) self))

(event EventOnPoolLeft
  (params (PopData :type Actor%20Pop%20Data%20Structure%20%28by%20ref%29))
  (bind (_owner _instigator _location _velocity _rotation _optionalobject _optionalobject2) (Utilities|Struct|BreakActorPopData PopData))
  (|CallParentFunction PopData)
  (Development|PrintText "Exiting Pool" true true "(R=0.000000,G=0.660000,B=1.000000,A=1.000000)" 0.2)
  (Utilities|FlowControl|Sequence
    (:then_0
      (bind _asrpg_ability_system_component (Utilities|Casting|CastToRPG_AbilitySystemComponent _optionalobject))
      (Variables|Default|SetRPGASC _asrpg_ability_system_component))
    (:then_1
      (bind _asrpg_gun_actor (Utilities|Casting|CastToRPG_GunActor _optionalobject2))
      (Variables|Default|SetGun%20Data (Variables|/Script/RPG.RPG_GunActor|GetGunData _asrpg_gun_actor)))))

(event EventLifeSpanExpired
  (Class|ActorPoolWorldSubsystem|AddActortoPool (Subsystems|GetActorPoolWorldSubsystem) self))

(event EventOnPoolEntered
  (|CallParentFunction)
  (Development|PrintText "Entering Pool" true true "(R=0.000000,G=0.660000,B=1.000000,A=1.000000)" 0.2))

(fn ConstructionScript)

(fn PlayImpactEffect
  (params (Hit%20Result :type Hit%20Result%20Structure))
  (bind _gun_data (Variables|Default|GetGun%20Data))
  (bind _weaponeffects (Variables|/Script/RPG.RPG_SuperGun|GetWeaponEffects _gun_data))
  (Utilities|IsValid _gun_data
    (:Is%20Valid
      (Utilities|IsValid _weaponeffects
        (:Is%20Valid
          (Class|RPGBFLMainFunctions|PlayEffectPackatLocation (Variables|/Script/RPG.RPG_WeaponEffectDataAsset|GetBulletImpactEffects _weaponeffects) self 0 "Instant" (Math|Transform|MakeTransform (.ImpactPoint (Collision|BreakHitResult Hit%20Result)) (Transformation|GetActorRotation) "1.000000,1.000000,1.000000")))))))

(fn AddImpulse
  (params (HitResult :type Hit%20Result%20Structure))
  (bind (_bblockinghit _binitialoverlap _time _distance _location _impactpoint _normal _impactnormal _physmat _hitactor _hitcomponent _hitbonename) (Collision|BreakHitResult HitResult))
  (if (Physics|IsSimulatingPhysics _hitcomponent _hitbonename)
    (Physics|AddImpulse _hitcomponent (* (Transformation|GetVelocity) (Variables|Default|GetMass)) _hitbonename false)))

(fn ApplyImpactDamage
  (params (HitActor :type Actor%20Object%20Reference) (HitResult :type Hit%20Result%20Structure))
  (Variables|Default|GetRPGASC
    (:then
      (bind _returnvalue (Class|RPGBFLMainFunctions|AddTargetDatatoContainerSpec (Variables|Default|GetEffectContainer) (Ability|TargetData|AbilityTargetDatafromHitResult HitResult)))
      (Class|RPGAbilitySystemComponent|ApplyGameplayEffectContainerSpec (Variables|Default|GetRPGASC) _returnvalue))
    (:else)))