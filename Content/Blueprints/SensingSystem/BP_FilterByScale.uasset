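; BP_FilterByScale is a sensing system filter that limits which target actors can be sensed, based on their size.
; It overrides K2_FilterActorsForSensing, looping over the candidate actors and keeping those whose world scale meets a hardcoded minimum on all three axes.
; The sensing component and owner inputs are unused, so the result depends only on each target's scale.
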(fn K2FilterActorsforSensing
  (params (SensingSystemComponent :type Sensing%20System%20Component%20Object%20Reference) (SensingSystemOwner :type Actor%20Object%20Reference) (TargetActors :type Array%20of%20Actor%20Object%20References))
  (for _array_element TargetActors
    (if (Math|Boolean|ANDBoolean (>= (.X (Math|Vector|BreakVector (Transformation|GetActorScale3D _array_element))) 3.0) (>= (.Y (Math|Vector|BreakVector (Transformation|GetActorScale3D _array_element))) 3.0) (>= (.Z (Math|Vector|BreakVector (Transformation|GetActorScale3D _array_element))) 3.0))
      (Utilities|Array|Add (LocalVariables|GetValidTargets) _array_element)))
  (return (LocalVariables|GetValidTargets)))