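; BP_Gun is an equippable gun weapon Blueprint that gives the equipping character an on-screen weapon info widget.
; EquipItem runs the parent logic, creates WBP_WeaponInfo for the character's player controller, sets it up with the gun, its GunData and the character's inventory component, then adds it to the viewport.
; UnEquipItem runs the parent logic and tears down the widget if it is still valid.
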(event EventBeginPlay)

(event Collision|EventActorBeginOverlap
  (params (OtherActor :type Actor%20Object%20Reference)))

(event EventTick
  (params (DeltaSeconds :type Float%20%28single-precision%29)))

(event EventEquipItem
  (params (EquippingCharacter :type RPG%20Character%20Object%20Reference) (RPGAbilitySystemComponent :type RPG%20Ability%20System%20Component%20Object%20Reference))
  (|CallParentFunction EquippingCharacter RPGAbilitySystemComponent)
  (bind _returnvalue (UserInterface|CreateWidget "/Game/UI/Weapons/WBP_WeaponInfo.WBP_WeaponInfo_C" (.AsPlayer%20Controller (Utilities|Casting|CastToPlayerController (Pawn|GetController EquippingCharacter)))))
  (bind _output_get (Variables|Default|SetWidget _returnvalue))
  (Default|SetupWidget _output_get self (Variables|Default|GetGunData) (Class|RPGCharacter|GetInventorySystemComponent EquippingCharacter))
  (UserInterface|Viewport|AddtoViewport (Variables|Default|GetWidget) 0))

(event EventUnEquipItem
  (params (EquippingCharacter :type RPG%20Character%20Object%20Reference) (RPGAbilitySystemComponent :type RPG%20Ability%20System%20Component%20Object%20Reference))
  (|CallParentFunction EquippingCharacter RPGAbilitySystemComponent)
  (bind _widget (Variables|Default|GetWidget)
    (:then
      (Default|TearDownWidget _widget))
    (:else)))

(fn ConstructionScript)