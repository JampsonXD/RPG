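; BP_SuperController is a player controller that owns the player's inventory component and its on-screen UI.
; On begin play it creates a hidden WBP_Inventory widget from the component's items and initializes the component, whose item-added event refreshes the widget.
; Pressing I toggles inventory visibility via a FlipFlop, while keys 1 and 2 add a chest or health potion.
; A separate CreateHUD event builds the HUD widget.
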(event OnItemAdded(InventorySystemComponent)
  (params (NewItem :type Item%20Object%20Reference))
  (Default|RefreshInventory (Variables|Default|GetInventoryWidget) (.OutItems (Class|InventorySystemComponent|GetInventoryItems (Variables|Default|GetInventorySystemComponent)))))

(event Custom|AddNewItem
  (params (ItemClass :type Item%20Class%20Reference) (StacksToGrant :type Integer))
  (Class|InventorySystemComponent|AddItem (Variables|Default|GetInventorySystemComponent) ItemClass StacksToGrant))

(event Custom|CreateHUD
  (bind _returnvalue (UserInterface|CreateWidget "/Game/UI/HUD.HUD_C" self))
  (bind _output_get (Variables|Default|SetHUD _returnvalue))
  (UserInterface|Viewport|AddtoViewport _output_get 0))

(event EventBeginPlay
  (|CallParentFunction)
  (CallFunction|CreateInventoryWidget)
  (Class|InventorySystemComponent|InitInventorySystemComponent (Variables|Default|GetInventorySystemComponent)))

(event Input|KeyboardEvents|1
  (params (Key :type Key%20Structure :default "None"))
  (:Pressed
    (CallFunction|AddNewItem "/Game/Items/Armor/BP_Chest.BP_Chest_C" 1)))

(event Input|KeyboardEvents|2
  (params (Key :type Key%20Structure :default "None"))
  (:Pressed
    (CallFunction|AddNewItem "/Game/Blueprints/Items/HealthPotion.HealthPotion_C" 1)))

(event Input|KeyboardEvents|I
  (params (Key :type Key%20Structure :default "None"))
  (:Pressed
    (bind _isa (Utilities|FlowControl|FlipFlop)
      (:A
        _)
      (:B
        _))
    (Widget|SetVisibility (Variables|Default|GetInventoryWidget) (select _isa "Visible" "Hidden"))))

(fn ConstructionScript)

(fn CreateInventoryWidget
  (bind _returnvalue (UserInterface|CreateWidget "/Game/UI/WBP_Inventory.WBP_Inventory_C" self (.OutItems (Class|InventorySystemComponent|GetInventoryItems (Variables|Default|GetInventorySystemComponent)))))
  (bind _output_get (Variables|Default|SetInventoryWidget _returnvalue))
  (UserInterface|Viewport|AddtoViewport _output_get 0)
  (Widget|SetVisibility _output_get "Hidden"))