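; Targeting type that finds targets in front of a character with a multi sphere trace, overriding GetTargets.
; The sweep runs from the character's eye view point along its view direction for a configurable distance, ignoring the targeting actor.
; Radius, channel, complex tracing and debug drawing come from variables, and all hit results are returned when the trace reports a hit.
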(fn GetTargets
  (params (TargetingCharacter :type RPG%20Character%20Object%20Reference) (TargetingActor :type Actor%20Object%20Reference) (EventData :type Gameplay%20Event%20Data%20Structure))
  (bind (_outlocation _outrotation) (Actor|GetActorEyesViewPoint TargetingCharacter))
  (bind (_outhits _returnvalue) (Collision|MultiSphereTraceByChannel TargetingCharacter _outlocation (+ _outlocation (* (Math|Vector|GetForwardVector _outrotation) (Variables|Default|GetForwardValue))) (Variables|Default|GetRadius) (Variables|Default|GetTrace%20Channel) (Variables|Default|GetTrace%20Complex) (Utilities|Array|MakeArray TargetingActor) (Variables|Default|GetDraw%20Debug%20Type) true (Variables|Default|GetTrace%20Color) (Variables|Default|GetTrace%20Hit%20Color) (Variables|Default|GetDraw%20Time)))
  (if _returnvalue
    (return _outhits 0)))