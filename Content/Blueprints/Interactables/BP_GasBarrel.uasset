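; BP_GasBarrel is an explosive barrel that blows up when it takes point or radial damage.
; Point damage detonates it at once, while radial damage waits a short random delay, staggering chain reactions.
; The explosion plays an effect pack, sphere-traces a random radius with debug drawing, forwards radial damage messages and applies a GAS damage effect to hit actors.
; It then calls CallFinished on itself; its pool enter and leave events are empty.
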(event Custom|Explode
  (params (Start :type Vector) (Radius :type Float%20%28single-precision%29))
  (Class|RPGBFLMainFunctions|PlayEffectPackatLocation (Variables|Default|GetExplosionPack) self 0 "Instant" (Math|Transform|MakeTransform Start "0, 0, 0" "1.000000,1.000000,1.000000"))
  (bind _outhits (Collision|MultiSphereTraceForObjects Start Start Radius (Utilities|Array|MakeArray "ObjectTypeQuery8" "ObjectTypeQuery7" "ObjectTypeQuery4") false 0 "ForDuration"))
  (for _array_element _outhits
    (Class|DamageableInterface|OnRadialDamage(Message) (.HitActor (Collision|BreakHitResult _array_element)))
    (Utilities|IsValid (Ability|GetAbilitySystemComponent (.HitActor (Collision|BreakHitResult _array_element)))
      (:Is%20Valid
        (GameplayEffects|ApplyGameplayEffectToTarget :self (Ability|GetAbilitySystemComponent (.HitActor (Collision|BreakHitResult _array_element))) :GameplayEffectClass "/Game/Characters/Global/GE/GE_PrimaryAttackDamage.GE_PrimaryAttackDamage_C" :Target (Ability|GetAbilitySystemComponent (.HitActor (Collision|BreakHitResult _array_element)))))))
  (Default|CallFinished self))

(event EventBeginPlay)

(event Collision|EventActorBeginOverlap
  (params (OtherActor :type Actor%20Object%20Reference)))

(event EventOnPoolLeft
  (params (PopData :type Actor%20Pop%20Data%20Structure%20%28by%20ref%29)))

(event EventOnPoolEntered)

(event EventOnRadialDamage
  (Utilities|FlowControl|Delay (Math|Random|RandomFloatinRange 0.3 0.6))
  (CallFunction|Explode (Transformation|GetActorLocation) (Math|Random|RandomFloatinRange 4e+02 6e+02)))

(event EventOnPointDamage
  (CallFunction|Explode (Transformation|GetActorLocation) (Math|Random|RandomFloatinRange 4e+02 6e+02)))

(event EventTick
  (params (DeltaSeconds :type Float%20%28single-precision%29)))

(fn ConstructionScript)