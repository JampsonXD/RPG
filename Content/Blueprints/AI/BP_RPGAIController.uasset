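; AI controller for RPG characters that drives behavior through a Behavior Tree and Blackboard.
; StartLogic initializes the Blackboard, runs the tree and starts the brain component, while StopLogic halts it with a given reason.
; AI perception updates write the player character to the "Target" key when sensed and clear it when sensing is lost, ignoring other actors.
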(event OnTargetPerceptionUpdated(AIPerception)
  (params (Actor :type Actor%20Object%20Reference) (Stimulus :type AI%20Stimulus%20Structure))
  (if (== Actor (Game|GetPlayerCharacter 0))
    (AI|Components|Blackboard|SetValueasObject (Variables|Default|GetBlackboard) (Utilities|Name|MakeLiteralName "Target") (Utilities|SelectObject Actor 0 (.bSuccessfullySensed (Utilities|Struct|BreakAIStimulus Stimulus))))))

(event Custom|StartLogic
  (Class|AIController|UseBlackboard (Variables|AIController|GetBlackboard%20Asset))
  (AI|RunBehaviorTree (Variables|AIController|GetBT%20Asset))
  (AI|Logic|StartLogic (Variables|Default|GetBrainComponent)))

(event Custom|Stop%20Logic
  (params (Reason :type String))
  (bind _braincomponent (Variables|Default|GetBrainComponent)
    (:then
      (AI|Logic|StopLogic _braincomponent Reason))
    (:else)))

(event EventBeginPlay)

(event EventTick
  (params (DeltaSeconds :type Float%20%28single-precision%29)))

(fn ConstructionScript)