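; Pooled zombie AI character that handles its own death and reuse through an actor pool.
; On death it tags itself Status.Dead, stops its BP_RPGAIController logic, removes its default ability set and enters the pool; leaving the pool reverses this.
; The corpse is a separately spawned PhysicsSkeletalMeshActor, given a pose snapshot, the mesh, a ragdoll AnimBP and the zombie's velocity as impulse.
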(event EventDeathEvent
  (Class|RPGBFLMainFunctions|AddLooseGameplayTagstoActor self "(GameplayTags=((TagName=\"Status.Dead\")))")
  (CallFunction|CreatePhysicsRagdoll)
  (Default|StopLogic (CallFunction|GetRPGAIController) "Entered Pool")
  (Class|RPGCharacter|RemoveDefaultAbilitySet)
  (Class|RPGBFLMainFunctions|AddActortoPool self))

(event EventOnPoolLeft
  (params (PopData :type Actor%20Pop%20Data%20Structure%20%28by%20ref%29))
  (Class|RPGCharacter|AddDefaultAbilitySet)
  (Class|RPGBFLMainFunctions|RemoveLooseGameplayTagstoActor self "(GameplayTags=((TagName=\"Status.Dead\")))")
  (Default|StartLogic (CallFunction|GetRPGAIController)))

(fn ConstructionScript)

(fn IsDead
  (return (GameplayTags|HasMatchingGameplayTag "(TagName=\"Status.Dead\")")))

(fn CreatePhysicsRagdoll
  (bind _mesh (Variables|Character|GetMesh))
  (bind _output_get (LocalVariables|SetTemp (Utilities|Struct|MakePoseSnapshot)))
  (Class|SkeletalMeshComponent|SnapshotPose (Variables|Character|GetMesh) _output_get)
  (Game|SpawnActorfromClass "/Game/Blueprints/Misc/PhysicsSkeletalMeshActor.PhysicsSkeletalMeshActor_C" (Transformation|GetWorldTransform _mesh) "AlwaysSpawn" 0 (LocalVariables|GetTemp) "/Game/Assets/BSP_ZombieAnims/Blueprints/ABP_Ragdoll_Zombie.ABP_Ragdoll_Zombie_C" (Variables|/Script/Engine.SkeletalMeshComponent|GetSkeletalMeshAsset _mesh) (Transformation|GetVelocity) 0))

(fn GetRPGAIController
  (return (.AsBP%20RPGAIController (Utilities|Casting|CastToBP_RPGAIController (Pawn|GetController)))))