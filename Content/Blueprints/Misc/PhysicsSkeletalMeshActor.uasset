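; Skeletal mesh actor that simulates physics from BeginPlay and removes itself once out of the player's way, like a disposable ragdoll or debris piece.
; The construction script calls an all-bodies impulse before assigning the configurable mesh and anim class, with physics simulation only enabled later at BeginPlay.
; A looping five-second timer destroys the actor when it is beyond a set distance from the player and has not been recently rendered.
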(event Custom|Cleanup
  (if (> (Transformation|GetDistanceTo (Game|GetPlayerCharacter 0)) 5e+02)
    (if (not (Class|Actor|WasRecentlyRendered 0.2))
      (Actor|DestroyActor))))

(event EventBeginPlay
  (Physics|SetSimulatePhysics (Variables|SkeletalMeshActor|GetSkeletalMeshComponent) true)
  (Utilities|Time|SetTimerbyEvent (delegate Custom|Cleanup) 5.0 true))

(fn ConstructionScript
  (Class|SkeletalMeshComponent|AddImpulsetoAllBodiesBelow (Variables|SkeletalMeshActor|GetSkeletalMeshComponent) (Variables|Default|GetImpulse) "None" false true)
  (Components|SkeletalMesh|SetSkeletalMeshAsset (Variables|SkeletalMeshActor|GetSkeletalMeshComponent) (Variables|Default|GetSkeletalMesh))
  (Class|SkeletalMeshComponent|SetAnimClass (Variables|SkeletalMeshActor|GetSkeletalMeshComponent) (Variables|Default|GetAnimationClass)))